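; Behavior tree decorator that detects whether any actor of the listed classes is within a set distance of the AI's pawn.
; It scans all actors of each class in turn and writes the first one in range, not necessarily the nearest, to the blackboard.
; It passes and enables AttackMode only if the pawn is a BaseDefender; otherwise, or with nothing in range, it fails.
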(fn PerformConditionCheckAI
  (params (OwnerController :type AI%20Controller%20Object%20Reference) (ControlledPawn :type Pawn%20Object%20Reference))
  (for _array_element (Variables|Default|GetActorToDetect)
    (bind _outactors (Actor|GetAllActorsOfClass _array_element))
    (for _array_element_2 _outactors
      (if (<= (Transformation|GetDistanceTo _array_element_2 ControlledPawn) (Variables|Default|GetDistance))
        (Class|BTFunctionLibrary|SetBlackboardValueasObject (Variables|Default|GetActorDetected) _array_element_2)
        (bind _asbase_defender (Utilities|Casting|CastToBaseDefender ControlledPawn)
          (:then
            (Variables|/Script/Mobile_TPS_INH.BaseDefender|SetbAttackMode _asbase_defender true)
            (return true))
          (:CastFailed
            (return false))))))
  (return false))