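; BP_Eater is an enemy that attacks a target with fireballs and has clamped health.
; BeginPlay caches its ABP_Eater anim instance, whose Attack flag is set by the Attack event.
; SpawnFireBall launches BP_FireBall from the jaw socket toward TargetActor and applies damage to it immediately, independent of any projectile hit.
; Health starts full in the construction script, and AnyDamage calls Die at zero.
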(event Custom|Attack
  ;[1 1 1] Atttack
  (Variables|/Game/Blueprints/Blueprint_Christophe/_Enemy/Eater/Animation/ABP_Eater.ABP_Eater_C|SetbAttack (Variables|Default|GetAs%20ABP%20Eater) true))

(event Custom|SpawnFireBall
  (bind _targetactor (Variables|Default|GetTargetActor))
  ;[1 1 1] SpawnFireBallProjectile
  (Game|SpawnActorfromClass "/Game/Blueprints/Blueprint_Christophe/_Enemy/Eater/BP_FireBall.BP_FireBall_C" (Math|Transform|MakeTransform (Transformation|GetSocketLocation (Variables|Character|GetMesh) "JawSocket") (Math|Rotator|FindLookatRotation (Transformation|GetActorLocation) (Transformation|GetActorLocation _targetactor)) "1.000000,1.000000,1.000000") "AlwaysSpawn" "MultiplyWithRoot" 0 0)
  (Game|Damage|ApplyDamage _targetactor 1e+01 0 0))

(event Game|Damage|EventAnyDamage
  (params (Damage :type Float%20%28single-precision%29) (DamageType :type Damage%20Type%20Object%20Reference) (InstigatedBy :type Controller%20Object%20Reference) (DamageCauser :type Actor%20Object%20Reference))
  ;[1 1 1] TakeDamage
  (bind _output_get (Variables|Default|SetHealth (Math|Float|Clamp(Float) (- (Variables|Default|GetHealth) Damage) 0.0 (Variables|Default|GetMaxHealth))))
  (if (<= _output_get 0.0)
    (Class|EnemyBase|Die)))

(event EventBeginPlay
  ;[1 1 1] Get Enemy AnimationBlueprint
  (bind _asabp_eater (Utilities|Casting|CastToABP_Eater (Components|SkeletalMesh|GetAnimInstance (Variables|Character|GetMesh))))
  (Variables|Default|SetAs%20ABP%20Eater _asabp_eater))

(fn ConstructionScript
  (bind _output_get (Variables|Default|SetMaxHealth 1e+02))
  (Variables|Default|SetHealth _output_get))