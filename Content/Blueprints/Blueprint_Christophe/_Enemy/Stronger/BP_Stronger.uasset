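; Stronger enemy Blueprint that handles a mouth attack, damage intake and death.
; On BeginPlay it caches its mesh's ABP_Eater anim instance.
; Attack plays the mouth montage and applies fixed damage to TargetActor only when the montage completes, with no range check.
; Health starts at the maximum set in the construction script, drops with clamping on any damage, and calls Die at zero.
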(event Custom|Attack
  ;[1 1 1] Attack
  (Animation|Montage|PlayMontage (Variables|Character|GetMesh) "/Game/0_Assets/Assets_Christophe/_Enemies/Dragons/Animations/DragonTheNightmare/AttackMouthAnim_Montage.AttackMouthAnim_Montage"
    (:OnCompleted
      (Game|Damage|ApplyDamage (Variables|Default|GetTargetActor) 3e+01 0 0))))

(event Game|Damage|EventAnyDamage
  (params (Damage :type Float%20%28single-precision%29) (DamageType :type Damage%20Type%20Object%20Reference) (InstigatedBy :type Controller%20Object%20Reference) (DamageCauser :type Actor%20Object%20Reference))
  ;[1 1 1] TakeDamage
  (bind _output_get (Variables|Default|SetHealth (Math|Float|Clamp(Float) (- (Variables|Default|GetHealth) Damage) 0.0 (Variables|Default|GetMaxHealth))))
  (if (<= _output_get 0.0)
    (Class|EnemyBase|Die)))

(event EventBeginPlay
  ;[1 1 1] Get Enemy AnimationBlueprint
  (bind _asabp_eater (Utilities|Casting|CastToABP_Eater (Components|SkeletalMesh|GetAnimInstance (Variables|Character|GetMesh))))
  (Variables|Default|SetAs%20ABP%20Eater _asabp_eater))

(fn ConstructionScript
  (bind _output_get (Variables|Default|SetMaxHealth 1e+02))
  (Variables|Default|SetHealth _output_get))