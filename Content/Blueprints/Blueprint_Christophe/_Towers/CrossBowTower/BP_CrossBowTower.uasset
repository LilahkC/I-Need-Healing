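; Crossbow tower that automatically fires arrows at enemies.
; It searches for an enemy on BeginPlay and after each shot, and turns the crossbow body toward a valid target every Tick.
; A Delay inside Tick paces the shots, each spawning a scaled-down BP_Arrow at the fire point, rotated toward the target.
; The construction script looks up the tower cost and takes a hardcoded amount of gold.
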(event EventBeginPlay
  (CallFunction|SearchEnemy))

(event EventTick
  (params (DeltaSeconds :type Float%20%28single-precision%29))
  (bind _returnvalue (Transformation|GetActorLocation))
  (bind _attacktarget (Variables|Default|GetAttackTarget))
  (bind _returnvalue_2 (Transformation|GetActorLocation _attacktarget))
  (bind _returnvalue_3 (Utilities|IsValid _attacktarget))
  (bind _returnvalue_4 (Math|Rotator|FindLookatRotation _returnvalue _returnvalue_2))
  (if _returnvalue_3
    (Transformation|SetRelativeRotation (Variables|Default|GetCrossBowBody) (Math|Rotator|MakeRotator (- (.roll _returnvalue_4) -1e+01) 0.0 (- (.yaw _returnvalue_4) 9e+01)) false false)
    (CallFunction|Attack)
    (Utilities|FlowControl|Delay 0.5)
    (if _returnvalue_3
      (Game|SpawnActorfromClass "/Game/Blueprints/Blueprint_Christophe/_Towers/CrossBowTower/BP_Arrow.BP_Arrow_C" (Math|Transform|MakeTransform (Transformation|GetSocketLocation (Variables|Default|GetFirePoint) "None") (Math|Rotator|MakeRotator (.roll _returnvalue_4) (.pitch _returnvalue_4) (.yaw _returnvalue_4)) "0.300000,0.300000,0.300000") "AlwaysSpawn" "MultiplyWithRoot" 0 0)
      (CallFunction|SearchEnemy))))

(fn ConstructionScript
  (Class|TowerBase|GetTowerCost "CrossBowTower")
  (Class|TowerBase|TakeGold 150))