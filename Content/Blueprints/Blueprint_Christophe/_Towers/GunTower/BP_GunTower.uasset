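; Gun tower that turns its upper turret toward an enemy target and fires bullets alternately from two barrels.
; BeginPlay calls SearchEnemy; while AttackTarget is valid, Tick updates the turret yaw and uses an AttackSpeed Delay to pace shots.
; A looping MultiGate alternates right and left fire points, each spawning an effect, an explosion sound at world origin and an aimed BP_Bullet.
; The construction script calls GetTowerCost and deducts a fixed amount of gold.
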(event EventBeginPlay
  (CallFunction|SearchEnemy))

(event EventTick
  (params (DeltaSeconds :type Float%20%28single-precision%29))
  (bind _firepoint_right (Variables|Default|GetFirePoint_Right))
  (bind _firepoint_left (Variables|Default|GetFirePoint_Left))
  (bind _attacktarget (Variables|Default|GetAttackTarget))
  (bind _returnvalue (Transformation|GetWorldLocation _firepoint_right))
  (bind _returnvalue_2 (Transformation|GetWorldLocation _firepoint_left))
  (if (Utilities|IsValid _attacktarget)
    (bind _output_get (Variables|Default|SetTargetLocation (Transformation|GetActorLocation _attacktarget)))
    (Transformation|SetRelativeRotation (Variables|Components|GetSM_UpperTurret) (Math|Rotator|MakeRotator 0.0 0.0 (- (.yaw (Math|Rotator|FindLookatRotation (Transformation|GetActorLocation) _output_get)) 9e+01)) false false)
    (Utilities|FlowControl|Delay (Variables|Default|GetAttackSpeed))
    (Utilities|FlowControl|MultiGate false true -1
      (:Out%200
        (Niagara|SpawnSystematLocation 0 _returnvalue)
        (Audio|SpawnSoundatLocation "/Game/StarterContent/Audio/Explosion01.Explosion01" "0, 0, 0" "0, 0, 0" 0.1 1.0 0.0 0 0)
        (Game|SpawnActorfromClass "/Game/Blueprints/Blueprint_Christophe/_Towers/GunTower/BP_Bullet.BP_Bullet_C" (Math|Transform|MakeTransform _returnvalue (Math|Rotator|MakeRotator (.roll (Math|Rotator|FindLookatRotation _returnvalue (Variables|Default|GetTargetLocation))) (.pitch (Math|Rotator|FindLookatRotation _returnvalue (Variables|Default|GetTargetLocation))) (.yaw (Math|Rotator|FindLookatRotation _returnvalue (Variables|Default|GetTargetLocation)))) "1.000000,1.000000,1.000000") "Undefined" "MultiplyWithRoot" 0 0))
      (:Out%201
        (Niagara|SpawnSystematLocation 0 _returnvalue_2)
        (Audio|SpawnSoundatLocation "/Game/StarterContent/Audio/Explosion02.Explosion02" "0, 0, 0" "0, 0, 0" 0.1 1.0 0.0 0 0)
        (Game|SpawnActorfromClass "/Game/Blueprints/Blueprint_Christophe/_Towers/GunTower/BP_Bullet.BP_Bullet_C" (Math|Transform|MakeTransform _returnvalue_2 (Math|Rotator|MakeRotator (.roll (Math|Rotator|FindLookatRotation _returnvalue_2 (Variables|Default|GetTargetLocation))) (.pitch (Math|Rotator|FindLookatRotation _returnvalue_2 (Variables|Default|GetTargetLocation))) (.yaw (Math|Rotator|FindLookatRotation _returnvalue_2 (Variables|Default|GetTargetLocation)))) "1.000000,1.000000,1.000000") "Undefined" "MultiplyWithRoot" 0 0)))))

(fn ConstructionScript
  (Class|TowerBase|GetTowerCost "GunTower")
  (Class|TowerBase|TakeGold 300))