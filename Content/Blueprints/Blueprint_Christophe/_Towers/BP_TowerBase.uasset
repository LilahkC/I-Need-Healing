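; Base tower actor that automatically targets enemies within its attack range, prioritizing the one closest to the allied base.
; A self-restarting search event runs a delayed multi-sphere object trace to collect EnemyBase actors around the tower.
; EnemyToBaseDistance compares their distances to the control point base found on BeginPlay.
; The selected target goes to an empty Attack event, apparently left for child towers to implement.
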(event Custom|SearchEnemy
  (bind _returnvalue (Transformation|GetActorLocation))
  ;[1 1 1] SearchEnemyInAttackRange
  (Utilities|FlowControl|Delay 0.3)
  (bind (_outhits _returnvalue_2) (Collision|MultiSphereTraceForObjects _returnvalue _returnvalue (Variables|Default|GetAttackRange) (Utilities|Array|MakeArray "ObjectTypeQuery7") false 0 "None" true "(R=1.000000,G=1.000000,B=1.000000,A=1.000000)" "(R=1.000000,G=1.000000,B=1.000000,A=1.000000)" 0.0))
  (if _returnvalue_2
    (Utilities|Array|Clear (Variables|Gaming|GetEnemyArray))
    (for _array_element _outhits
      (bind _asenemy_base (Utilities|Casting|CastToEnemyBase (.HitActor (Collision|BreakHitResult _array_element))))
      (Utilities|Array|Add (Variables|Gaming|GetEnemyArray) _asenemy_base))
    (if (>= (Utilities|Array|Length (Variables|Gaming|GetEnemyArray)) 1)
      (bind (_hasenemy _nearestenemytoattack) (CallFunction|EnemytoBaseDistance))
      (if _hasenemy
        (bind _output_get (Variables|Default|SetAttackTarget _nearestenemytoattack))
        (CallFunction|Attack _output_get)
        (CallFunction|SearchEnemy)
        (else
          (CallFunction|SearchEnemy :!label _label)))
      (else
        (goto _label)))
    (else
      (CallFunction|SearchEnemy)
      (Variables|Default|SetAttackTarget 0))))

(event Custom|Attack
  (params (AttackTarget :type Enemy%20Base%20Object%20Reference))
  ;[1 1 1] Attack
)

(event EventBeginPlay
  ;[1 1 1] GetOurBase
  (CallFunction|SearchEnemy)
  (bind _returnvalue (Actor|GetActorOfClass "/Game/Blueprints/Blueprint_Christophe/Environment/BP_ControlPointBase.BP_ControlPointBase_C"))
  (Variables|Default|SetAlineBase _returnvalue))

(fn ConstructionScript)

(fn EnemytoBaseDistance
  (for _array_element (Variables|Gaming|GetEnemyArray)
    (if (<= (Math|Vector|VectorLength (- (Transformation|GetActorLocation (Variables|Default|GetAlineBase)) (Transformation|GetActorLocation _array_element))) (LocalVariables|GetEnemyDistanceTmp))
      (LocalVariables|SetEnemyDistanceTmp (Math|Vector|VectorLength (- (Transformation|GetActorLocation (Variables|Default|GetAlineBase)) (Transformation|GetActorLocation _array_element))))
      (LocalVariables|SetNearestEnemyTmp _array_element)))
  (return (Utilities|IsValid (LocalVariables|GetNearestEnemyTmp)) (LocalVariables|GetNearestEnemyTmp)))