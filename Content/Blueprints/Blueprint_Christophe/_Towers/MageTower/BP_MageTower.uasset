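; Mage tower for a tower defense game that damages its target with a continuous Niagara beam.
; BeginPlay calls SearchEnemy; Tick shows the beam ending at a valid AttackTarget and applies damage through a short Delay, otherwise hiding the beam.
; The construction script calls GetTowerCost, then takes a hard-coded amount of gold.
; A Timeline for spinning the gate and collectible meshes is present but never runs.
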(event EventBeginPlay
  (CallFunction|SearchEnemy))

(event EventTick
  (params (DeltaSeconds :type Float%20%28single-precision%29))
  (bind _attacktarget (Variables|Default|GetAttackTarget))
  (bind _ns_magebeam (Variables|Default|GetNS_MageBeam))
  ;[1 1 1] DoDamage
  (if (Utilities|IsValid _attacktarget)
    (Rendering|SetVisibility _ns_magebeam true false)
    (Class|NiagaraComponent|SetNiagaraVariableVec3 (Variables|Default|GetNS_MageBeam) "Beam_End" (Transformation|GetActorLocation _attacktarget))
    (Utilities|FlowControl|Delay 0.1)
    (Game|Damage|ApplyDamage (Variables|Default|GetAttackTarget) 1e+01 0 0)
    (else
      (Rendering|SetVisibility _ns_magebeam false false))))

(fn ConstructionScript
  (Class|TowerBase|GetTowerCost "MageTower")
  (Class|TowerBase|TakeGold 200))