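; BP_RockWall is an environment actor that builds a rock wall along a spline.
; Its construction script spreads a set count of static mesh components by distance along the spline in local space, setting only their location.
; Each component gets an unseeded random pick from the rock mesh array, so the layout can change whenever construction reruns.
; The event graph has no active logic.
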(event EventBeginPlay)

(event Collision|EventActorBeginOverlap
  (params (OtherActor :type Actor%20Object%20Reference)))

(event EventTick
  (params (DeltaSeconds :type Float%20%28single-precision%29)))

(fn ConstructionScript
  (bind _spline (Variables|Default|GetSpline))
  (for _index (range 0 (- (Variables|Default|GetCounts) 1))
    (bind _returnvalue (AddComponent|AddStaticMeshComponent false (Math|Transform|MakeTransform (Spline|GetLocationatDistanceAlongSpline _spline (* (/ _index (Variables|Default|GetCounts)) (Spline|GetSplineLength _spline)) "Local") "0, 0, 0" "1.000000,1.000000,1.000000")))
    (Components|StaticMesh|SetStaticMesh _returnvalue (.OutItem (Utilities|Array|Random (Variables|Default|GetRockMehes))))))