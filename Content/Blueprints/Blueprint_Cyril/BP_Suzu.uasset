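; BP_Suzu is an ability actor, modelled by name on Kiriko's Suzu, that grants defenders temporary invincibility in an area.
; Its Hit event hides the Suzu mesh, shows the sphere, resets the box's rotation and enables its overlaps, then destroys the actor after SuzuActiveTime.
; Any BaseDefender that begins overlapping the box becomes invincible for the full SuzuActiveTime, regardless of when it enters.
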(event OnComponentBeginOverlap(Box)
  (params (OverlappedComponent :type Primitive%20Component%20Object%20Reference) (OtherActor :type Actor%20Object%20Reference) (OtherComp :type Primitive%20Component%20Object%20Reference) (OtherBodyIndex :type Integer) (bFromSweep :type Boolean) (SweepResult :type Hit%20Result%20Structure%20%28by%20ref%29))
  (bind _asbase_defender (Utilities|Casting|CastToBaseDefender OtherActor))
  (Class|BaseCharacter|BecomeInvincible _asbase_defender (Variables|Default|GetSuzuActiveTime)))

(event OnComponentEndOverlap(Box)
  (params (OverlappedComponent :type Primitive%20Component%20Object%20Reference) (OtherActor :type Actor%20Object%20Reference) (OtherComp :type Primitive%20Component%20Object%20Reference) (OtherBodyIndex :type Integer)))

(event Collision|EventHit
  (params (MyComp :type Primitive%20Component%20Object%20Reference) (Other :type Actor%20Object%20Reference) (OtherComp :type Primitive%20Component%20Object%20Reference) (bSelfMoved :type Boolean) (HitLocation :type Vector :default "0, 0, 0") (HitNormal :type Vector :default "0, 0, 0") (NormalImpulse :type Vector :default "0, 0, 0") (Hit :type Hit%20Result%20Structure%20%28by%20ref%29))
  (bind _box (Variables|Default|GetBox))
  (Rendering|SetVisibility (Variables|Default|GetKiriko_Suzu) false false)
  (Rendering|SetVisibility (Variables|Default|GetSphere) true true)
  (Variables|/Script/Engine.PrimitiveComponent|SetbGenerateOverlapEvents _box true)
  (Transformation|SetRelativeRotation _box "0, 0, 0" false false)
  (Utilities|FlowControl|Delay (Variables|Default|GetSuzuActiveTime))
  (Actor|DestroyActor))

(fn ConstructionScript)