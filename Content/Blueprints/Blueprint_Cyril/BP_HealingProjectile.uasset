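; BP_HealingProjectile is a projectile that heals any BaseDefender it hits.
; On BeginPlay it copies its Speed variable into the ProjectileMovement component's InitialSpeed.
; On Hit it casts the other actor to BaseDefender and adds HealValue directly to its Health, clamped between zero and MaxHealth.
; The projectile destroys itself after any hit, whether or not the cast succeeds.
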(event EventBeginPlay
  (Variables|/Script/Engine.ProjectileMovementComponent|SetInitialSpeed (Variables|Default|GetProjectileMovement) (Variables|Default|GetSpeed)))

(event Collision|EventHit
  (params (MyComp :type Primitive%20Component%20Object%20Reference) (Other :type Actor%20Object%20Reference) (OtherComp :type Primitive%20Component%20Object%20Reference) (bSelfMoved :type Boolean) (HitLocation :type Vector :default "0, 0, 0") (HitNormal :type Vector :default "0, 0, 0") (NormalImpulse :type Vector :default "0, 0, 0") (Hit :type Hit%20Result%20Structure%20%28by%20ref%29))
  (bind _asbase_defender (Utilities|Casting|CastToBaseDefender Other)
    (:then
      (Variables|/Script/Mobile_TPS_INH.BaseCharacter|SetHealth _asbase_defender (Math|Float|Clamp(Float) (+ (Variables|/Script/Mobile_TPS_INH.BaseCharacter|GetHealth _asbase_defender) (Variables|Default|GetHealValue)) 0.0 (Variables|/Script/Mobile_TPS_INH.BaseCharacter|GetMaxHealth _asbase_defender)))
      (Actor|DestroyActor))
    (:CastFailed
      (Actor|DestroyActor))))

(fn ConstructionScript)